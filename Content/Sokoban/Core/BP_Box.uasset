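; BP_Box is the pushable crate in a Sokoban game, sliding across the grid when pushed.
; PlayMoveAnimation asks the grid manager whether the move is allowed, then a Timeline alpha offsets the box one cell from its start position.
; When the slide finishes it clears IsMoving and has the manager check for a win; a blocked push just clears the pushed box's IsMoving.
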(event Custom|PlayMoveAnimation
  (params (DirX :type Integer) (DirY :type Integer) (PushedBox :type BP%20Box%20Object%20Reference))
  (bind _gridmanagerref (Variables|Default|GetGridManagerRef))
  (bind _cellsize (Variables|/Game/Sokoban/Core/BP_GridManager.BP_GridManager_C|GetCellSize _gridmanagerref))
  (bind _bboxcanmove (Default|BoxMove _gridmanagerref DirX DirY PushedBox))
  (if _bboxcanmove
    (Variables|Default|SetBoxStartPos (Transformation|GetActorLocation PushedBox))
    (bind _move_alpha (Timeline|Timeline PlayFromStart)
      (:Update
        (Transformation|SetActorLocation (+ (* _move_alpha (Math|Vector|MakeVector (* DirX _cellsize) (* DirY _cellsize) 0.0)) (Variables|Default|GetBoxStartPos)) false false))
      (:Finished
        (Variables|Default|SetIsMoving false)
        (Default|CheckWin (Variables|Default|GetGridManagerRef))))
    (else
      (Variables|BP_Box_C|SetIsMoving PushedBox false))))

(event EventBeginPlay)

(event Collision|EventActorBeginOverlap
  (params (OtherActor :type Actor%20Object%20Reference)))

(event EventTick
  (params (DeltaSeconds :type Float%20%28single-precision%29)))

(fn ConstructionScript)