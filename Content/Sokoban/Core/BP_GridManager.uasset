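; Grid manager for a Sokoban level that builds the board, validates box pushes and detects victory.
; Level text comes from DT_Levels or game-instance custom/temp data by play mode, and InitLevel parses it into a cell map and position arrays.
; It respawns scaled box, wall and target actors and repositions the player.
; BoxMove updates logical box positions; CheckWin shows W_Victory and pauses when all boxes sit on targets.
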(event EventBeginPlay
  (bind _asgi_sokoban (Utilities|Casting|CastToGI_Sokoban (Game|GetGameInstance)))
  (bind _gridtext (CallFunction|GetLevelData (Variables|/Game/Sokoban/Core/GI_Sokoban.GI_Sokoban_C|GetCurrentLevelIndex _asgi_sokoban)))
  (CallFunction|InitLevel _gridtext))

(event Collision|EventActorBeginOverlap
  (params (OtherActor :type Actor%20Object%20Reference)))

(event EventTick
  (params (DeltaSeconds :type Float%20%28single-precision%29)))

(fn ConstructionScript)

(fn InitLevel
  (params (GridText :type String))
  (bind _cellsize (Variables|Default|GetCellSize))
  (bind _boxactors (Variables|Default|GetBoxActors))
  (bind _wallactors (Variables|Default|GetWallActors))
  (bind _targetactors (Variables|Default|GetTargetActors))
  (bind _cellsize_2 (Variables|Default|GetCellSize))
  (bind _cellsize_3 (Variables|Default|GetCellSize))
  (bind _cellsize_4 (Variables|Default|GetCellSize))
  (bind _returnvalue (* _cellsize 0.5))
  (bind _returnvalue_2 (* _cellsize_3 0.5))
  (bind _returnvalue_3 (/ _cellsize_2 1e+02))
  (bind _returnvalue_4 (/ _cellsize_3 1e+02))
  (bind _returnvalue_5 (/ _cellsize_4 1e+02))
  (Utilities|Array|Clear (Variables|Default|GetBoxPositions))
  (Utilities|Array|Clear (Variables|Default|GetWallPositions))
  (Utilities|Array|Clear (Variables|Default|GetTargetPositions))
  (Utilities|Map|Clear (Variables|Default|GetGridState))
  (for _index (range 0 (- (Utilities|String|Len GridText) 1))
    (switch string (Class|KismetStringLibrary|Mid GridText _index 1)
      (:Default
        (if (== (Utilities|String|GetCharacterasNumber (Class|KismetStringLibrary|Mid GridText _index 1)) 10)
          (LocalVariables|SetX 0)
          (LocalVariables|SetY (+ (LocalVariables|GetY) 1))))
      (:#
        (Utilities|Map|Add (Variables|Default|GetGridState) (Utilities|Struct|MakeIntPoint (LocalVariables|GetX) (LocalVariables|GetY)) "NewEnumerator1")
        (Utilities|Array|Add (Variables|Default|GetWallPositions) (Utilities|Struct|MakeIntPoint (LocalVariables|GetX) (LocalVariables|GetY)))
        (LocalVariables|SetX (+ (LocalVariables|GetX) 1)))
      (:-
        (Utilities|Map|Add (Variables|Default|GetGridState) (Utilities|Struct|MakeIntPoint (LocalVariables|GetX) (LocalVariables|GetY)) "NewEnumerator0")
        (LocalVariables|SetX (+ (LocalVariables|GetX) 1)))
      (:.
        (Utilities|Map|Add (Variables|Default|GetGridState) (Utilities|Struct|MakeIntPoint (LocalVariables|GetX) (LocalVariables|GetY)) "NewEnumerator2")
        (Utilities|Array|Add (Variables|Default|GetTargetPositions) (Utilities|Struct|MakeIntPoint (LocalVariables|GetX) (LocalVariables|GetY)))
        (LocalVariables|SetX (+ (LocalVariables|GetX) 1)))
      (:$
        (Utilities|Map|Add (Variables|Default|GetGridState) (Utilities|Struct|MakeIntPoint (LocalVariables|GetX) (LocalVariables|GetY)) "NewEnumerator0")
        (Utilities|Array|Add (Variables|Default|GetBoxPositions) (Utilities|Struct|MakeIntPoint (LocalVariables|GetX) (LocalVariables|GetY)))
        (LocalVariables|SetX (+ (LocalVariables|GetX) 1)))
      (:@
        (Utilities|Map|Add (Variables|Default|GetGridState) (Utilities|Struct|MakeIntPoint (LocalVariables|GetX) (LocalVariables|GetY)) "NewEnumerator0")
        (Variables|Default|SetPlayerStartPosition (Utilities|Struct|MakeIntPoint (LocalVariables|GetX) (LocalVariables|GetY)))
        (LocalVariables|SetX (+ (LocalVariables|GetX) 1)))
      (:+
        (Utilities|Map|Add (Variables|Default|GetGridState) (Utilities|Struct|MakeIntPoint (LocalVariables|GetX) (LocalVariables|GetY)) "NewEnumerator2")
        (Utilities|Array|Add (Variables|Default|GetTargetPositions) (Utilities|Struct|MakeIntPoint (LocalVariables|GetX) (LocalVariables|GetY)))
        (Variables|Default|SetPlayerStartPosition (Utilities|Struct|MakeIntPoint (LocalVariables|GetX) (LocalVariables|GetY)))
        (LocalVariables|SetX (+ (LocalVariables|GetX) 1)))
      (:*
        (Utilities|Map|Add (Variables|Default|GetGridState) (Utilities|Struct|MakeIntPoint (LocalVariables|GetX) (LocalVariables|GetY)) "NewEnumerator2")
        (Utilities|Array|Add (Variables|Default|GetTargetPositions) (Utilities|Struct|MakeIntPoint (LocalVariables|GetX) (LocalVariables|GetY)))
        (Utilities|Array|Add (Variables|Default|GetBoxPositions) (Utilities|Struct|MakeIntPoint (LocalVariables|GetX) (LocalVariables|GetY)))
        (LocalVariables|SetX (+ (LocalVariables|GetX) 1)))))
  (if (> (Utilities|Array|Length _boxactors) 0)
    (for _array_element _boxactors
      (Actor|DestroyActor _array_element))
    (Utilities|Array|Clear _boxactors))
  (if (> (Utilities|Array|Length _wallactors) 0)
    (for _array_element_2 _wallactors
      (Actor|DestroyActor _array_element_2))
    (Utilities|Array|Clear _wallactors))
  (if (> (Utilities|Array|Length _targetactors) 0)
    (for _array_element_3 _targetactors
      (Actor|DestroyActor _array_element_3))
    (Utilities|Array|Clear _targetactors))
  (for _array_element_4 (Variables|Default|GetBoxPositions)
    (bind _worldpos (CallFunction|GridtoWorld (.X (Utilities|Struct|BreakIntPoint _array_element_4)) (.Y (Utilities|Struct|BreakIntPoint _array_element_4))))
    (bind _returnvalue_6 (Game|SpawnActorfromClass "/Game/Sokoban/Core/BP_Box.BP_Box_C" (Math|Transform|MakeTransform _worldpos "0, 0, 0" (Math|Vector|MakeVector _returnvalue_3 _returnvalue_3 _returnvalue_3)) "AlwaysSpawn" "MultiplyWithRoot" 0 0))
    (Variables|/Game/Sokoban/Core/BP_Box.BP_Box_C|SetGridManagerRef _returnvalue_6 self)
    (Utilities|Array|Add (Variables|Default|GetBoxActors) _returnvalue_6))
  (for _array_element_5 (Variables|Default|GetWallPositions)
    (bind _worldpos_2 (CallFunction|GridtoWorld (.X (Utilities|Struct|BreakIntPoint _array_element_5)) (.Y (Utilities|Struct|BreakIntPoint _array_element_5))))
    (bind _returnvalue_7 (Game|SpawnActorfromClass "/Game/Sokoban/Core/BP_Wall.BP_Wall_C" (Math|Transform|MakeTransform _worldpos_2 "0, 0, 0" (Math|Vector|MakeVector _returnvalue_5 _returnvalue_5 _returnvalue_5)) "AlwaysSpawn" "MultiplyWithRoot" 0 0))
    (Utilities|Array|Add (Variables|Default|GetWallActors) _returnvalue_7))
  (for _array_element_6 (Variables|Default|GetTargetPositions)
    (bind _worldpos_3 (CallFunction|GridtoWorld (.X (Utilities|Struct|BreakIntPoint _array_element_6)) (.Y (Utilities|Struct|BreakIntPoint _array_element_6))))
    (bind _returnvalue_8 (Game|SpawnActorfromClass "/Game/Sokoban/Core/BP_Target.BP_Target_C" (Math|Transform|MakeTransform (+ _worldpos_3 (Math|Vector|MakeVector _returnvalue_2 _returnvalue_2 0.0)) "0, 0, 0" (Math|Vector|MakeVector _returnvalue_4 _returnvalue_4 _returnvalue_4)) "AlwaysSpawn" "MultiplyWithRoot" 0 0))
    (Utilities|Array|Add (Variables|Default|GetTargetActors) _returnvalue_8))
  (bind _worldpos_4 (CallFunction|GridtoWorld (.X (Utilities|Struct|BreakIntPoint (Variables|Default|GetPlayerStartPosition))) (.Y (Utilities|Struct|BreakIntPoint (Variables|Default|GetPlayerStartPosition)))))
  (Transformation|SetActorLocation (Variables|Default|GetPlayerActor) (+ _worldpos_4 (Math|Vector|MakeVector _returnvalue _returnvalue _returnvalue)) false false))

(fn CheckWin
  (for _array_element (Variables|Default|GetBoxPositions)
    (if (not (Utilities|Array|ContainsItem (Variables|Default|GetTargetPositions) _array_element))
      (return)))
  (bind _returnvalue (UserInterface|CreateWidget "/Game/Sokoban/UI/W_Victory.W_Victory_C"))
  (UserInterface|Viewport|AddtoViewport _returnvalue 0)
  (Game|SetGamePaused true))

(fn Reset
  (bind _asgi_sokoban (Utilities|Casting|CastToGI_Sokoban (Game|GetGameInstance)))
  (bind _gridtext (CallFunction|GetLevelData (Variables|/Game/Sokoban/Core/GI_Sokoban.GI_Sokoban_C|GetCurrentLevelIndex _asgi_sokoban)))
  (CallFunction|InitLevel _gridtext))

(fn GridtoWorld
  (params (GridX :type Integer) (GridY :type Integer))
  (bind _cellsize (Variables|Default|GetCellSize))
  (return (Math|Vector|MakeVector (* GridX _cellsize) (* GridY _cellsize) 0.0)))

(fn BoxMove
  (params (DirX :type Integer) (DirY :type Integer) (PushedBox :type BP%20Box%20Object%20Reference))
  (bind _intpoint (Utilities|Struct|MakeIntPoint DirX DirY))
  (bind _boxactors (Variables|Default|GetBoxActors))
  (bind _gridstate (Variables|Default|GetGridState))
  (bind _boxpositions (Variables|Default|GetBoxPositions))
  (bind _returnvalue (Utilities|Array|FindItem _boxactors PushedBox))
  (bind _output (Utilities|Array|Get(acopy) _boxpositions _returnvalue))
  (bind _returnvalue_2 (+ _intpoint _output))
  (bind (_value _returnvalue_3) (Utilities|Map|Find _gridstate _returnvalue_2))
  (if (Utilities|Array|ContainsItem (Variables|Default|GetBoxPositions) _returnvalue_2)
    _
    (elif _returnvalue_3
      (switch Utilities|FlowControl|Switch|SwitchonE_CellType _value
        (:NewEnumerator0
          (Utilities|Array|SetArrayElem (Variables|Default|GetBoxPositions) _returnvalue _returnvalue_2 :!label _label)
          (return true _returnvalue_2))
        (:NewEnumerator1
          _)
        (:NewEnumerator2
          (goto _label)))))
  (return false ""))

(fn GetLevelData
  (params (LevelIndex :type Integer))
  (bind _asgi_sokoban (Utilities|Casting|CastToGI_Sokoban (Game|GetGameInstance)))
  (switch int (Variables|/Game/Sokoban/Core/GI_Sokoban.GI_Sokoban_C|GetPlayMode _asgi_sokoban)
    (:0
      _)
    (:1
      _)
    (:2
      (return (.GridText (Utilities|Struct|BreakS_LevelData (Utilities|Array|Get(acopy) (Variables|/Game/Sokoban/Core/GI_Sokoban.GI_Sokoban_C|GetCustomLevels _asgi_sokoban) LevelIndex)))))
    (:3
      (return (.GridText (Utilities|Struct|BreakS_LevelData (Variables|/Game/Sokoban/Core/GI_Sokoban.GI_Sokoban_C|GetTempLevelData _asgi_sokoban))))))
  (bind _outrownames (DataTable|GetDataTableRowNames "/Game/Sokoban/Core/DT_Levels.DT_Levels"))
  (bind _returnvalue (Utilities|GetDataTableRow "/Game/Sokoban/Core/DT_Levels.DT_Levels" (Utilities|Array|Get(acopy) _outrownames LevelIndex))
    (:then
      (return (.GridText (Utilities|Struct|BreakS_LevelData _returnvalue))))))